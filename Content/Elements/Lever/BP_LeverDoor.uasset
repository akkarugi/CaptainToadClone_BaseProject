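; Lever actor that swings a door open and closed when Door_Interact fires while its prompt widget is visible.
; BeginPlay creates the hidden-or-shown BP_LeverDoorUI prompt, toggled by box overlap, and grabs a BP_Door via GetActorOfClass.
; A FlipFlop plays or reverses a Timeline that lerps door yaw to negative Rotation, with DoOnce blocking input until it finishes.
; OpenDoor and CloseDoor hold fixed-angle variants the event graph never calls.
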(event `Door_Interact`
  (if (`Widget.IsVisible` (`self.Canvas`))
    (`/Engine/EditorBlueprintResources/StandardMacros.DoOnce` false :!label _label
      (:`Completed`
        (`/Engine/EditorBlueprintResources/StandardMacros.FlipFlop`
          (:`A`
            (bind (_direction _floatvalue) (`Timeline|Timeline` :!via `PlayFromStart` :!label _label_2)
              (:`Update`
                (`SceneComponent.K2_SetRelativeRotation` (`/Game/Elements/BP_Door.door-rotate-large` (`self.DoorRef`)) (`KismetMathLibrary.MakeRotator` 0.0 0.0 (`KismetMathLibrary.Lerp` 0.0 (- 0.0 (`self.rotation`)) _floatvalue)) false false))
              (:`Finished`
                (goto _label :!via `Reset`))))
          (:`B`
            (goto _label_2 :!via `ReverseFromEnd`)))))))

(event `self.ReceiveBeginPlay`
  (bind _returnvalue (`|CreateWidget` "/Game/Elements/Lever/BP_LeverDoorUI.BP_LeverDoorUI_C"))
  (bind _output_get (set `self.Canvas` _returnvalue))
  (`UserWidget.AddToViewport` _output_get 0)
  (bind _returnvalue_2 (`GameplayStatics.GetActorOfClass` "/Game/Elements/BP_Door.BP_Door_C"))
  (set `self.DoorRef` _returnvalue_2))

(event `self.Box.OnComponentBeginOverlap`
  (params (OverlappedComponent :type "PrimitiveComponent Object Reference") (OtherActor :type "Actor Object Reference") (OtherComp :type "PrimitiveComponent Object Reference") (OtherBodyIndex :type Integer) (bFromSweep :type Boolean) (SweepResult :type "HitResult Structure (by ref)"))
  (`Widget.SetVisibility` (`self.Canvas`) "Visible"))

(event `self.Box.OnComponentEndOverlap`
  (params (OverlappedComponent :type "PrimitiveComponent Object Reference") (OtherActor :type "Actor Object Reference") (OtherComp :type "PrimitiveComponent Object Reference") (OtherBodyIndex :type Integer))
  (`Widget.SetVisibility` (`self.Canvas`) "Hidden"))

(fn `CloseDoor`
  (params (self2 :type "SceneComponent Object Reference") (Alpha :type "Float (double-precision)"))
  (`SceneComponent.K2_SetRelativeRotation` self2 (`KismetMathLibrary.MakeRotator` 0.0 0.0 (`KismetMathLibrary.Lerp` -90.0 0.0 Alpha)) false false))

(fn `OpenDoor`
  (params (Alpha :type "Float (double-precision)") (self2 :type "/Game/Elements/BP_Door Object Reference"))
  (returns (`door-rotate-large` :type "StaticMeshComponent Object Reference"))
  (bind _door_rotate_large (`/Game/Elements/BP_Door.door-rotate-large` self2))
  (`SceneComponent.K2_SetRelativeRotation` _door_rotate_large (`KismetMathLibrary.MakeRotator` 0.0 0.0 (`KismetMathLibrary.Lerp` 0.0 -90.0 Alpha)) false false)
  (return _door_rotate_large))

(fn `UserConstructionScript`)