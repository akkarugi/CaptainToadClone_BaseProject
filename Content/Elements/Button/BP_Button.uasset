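; Button actor whose Box trigger rotates the platforms of two bridges, BP_AdditiveBridge and BP_NoAdditiveBridge, found by class at BeginPlay.
; Any begin overlap adds the Rotation variable as local yaw to both platforms.
; End overlap adds the same yaw, not its inverse, to the non-additive bridge only.
; Timeline-driven rotation logic is left unconnected, and both bridge custom events are empty.
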(event `NoAditiveBridge`)

(event `AdditiveBridge`)

(event `self.ReceiveBeginPlay`
  (bind _returnvalue (`GameplayStatics.GetActorOfClass` "/Game/Elements/BP_AdditiveBridge.BP_AdditiveBridge_C"))
  (bind _output_get (set `self.AddititiveBridge` _returnvalue))
  (bind _returnvalue_2 (`GameplayStatics.GetActorOfClass` "/Game/Elements/BP_NoAdditiveBridge.BP_NoAdditiveBridge_C"))
  (bind _output_get_2 (set `self.NoAdditiveBridge` _returnvalue_2)))

(event `self.Box.OnComponentBeginOverlap`
  (params (OverlappedComponent :type "PrimitiveComponent Object Reference") (OtherActor :type "Actor Object Reference") (OtherComp :type "PrimitiveComponent Object Reference") (OtherBodyIndex :type Integer) (bFromSweep :type Boolean) (SweepResult :type "HitResult Structure (by ref)"))
  (bind __rotation (`self.-Rotation`))
  (`SceneComponent.K2_AddLocalRotation` (`/Game/Elements/BP_AdditiveBridge.platform` (stale `self.ReceiveBeginPlay` _output_get)) (`KismetMathLibrary.MakeRotator` 0.0 0.0 __rotation) false false)
  (`SceneComponent.K2_AddLocalRotation` (`/Game/Elements/BP_NoAdditiveBridge.platform` (stale `self.ReceiveBeginPlay` _output_get_2)) (`KismetMathLibrary.MakeRotator` 0.0 0.0 __rotation) false false))

(event `self.Box.OnComponentEndOverlap`
  (params (OverlappedComponent :type "PrimitiveComponent Object Reference") (OtherActor :type "Actor Object Reference") (OtherComp :type "PrimitiveComponent Object Reference") (OtherBodyIndex :type Integer))
  (`SceneComponent.K2_AddLocalRotation` (`/Game/Elements/BP_NoAdditiveBridge.platform` (stale `self.ReceiveBeginPlay` _output_get_2)) (`KismetMathLibrary.MakeRotator` 0.0 0.0 (`self.+Rotation`)) false false))

(fn `UserConstructionScript`)